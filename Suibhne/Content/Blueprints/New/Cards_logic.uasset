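; Cards_logic is a card-game logic Blueprint that generates a hand as an array of integers.
; GenerateHand divides CardsCounter by CardTypeCounter, then loops over half that value to fill TempHand with pairs.
; Each pair is a random integer below the per-type count and its complement to that count.
; The event graph and construction script are empty, and TempAcc is reset but otherwise unused.
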(event EventBeginPlay)

(event EventTick
  (params (DeltaSeconds :type Float%20%28single-precision%29)))

(fn ConstructionScript)

(fn GenerateHand
  (bind _cardtypecounter (Variables|Default|GetCardTypeCounter))
  (bind _temphand (Variables|Default|GettempHand))
  (bind _cardscounter (Variables|Default|GetCardsCounter))
  (bind _returnvalue (/ _cardscounter _cardtypecounter))
  (Variables|Default|SetTempAcc 0)
  (Variables|Default|SetCardsByTypeCounter _returnvalue)
  (Utilities|Array|Clear _temphand)
  (for _index (range 0 (/ _returnvalue 2))
    (bind _returnvalue_2 (Utilities|Array|Add _temphand (Math|Random|RandomInteger (Variables|Default|GetCardsByTypeCounter))))
    (Utilities|Array|Add _temphand (- (Variables|Default|GetCardsByTypeCounter) (Utilities|Array|Get(acopy) _temphand _returnvalue_2))))
  (return _temphand))